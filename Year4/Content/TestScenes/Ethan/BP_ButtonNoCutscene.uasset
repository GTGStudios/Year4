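; A button Blueprint that, once a key is picked up, opens the BP_DoorAnim1 doors whose DoorValue matches its ButtonValue.
; StartInteract searches all such doors, calls OpenDoor with the player character on each match and sets the player's view target to that door.
; A successful match blocks further use, while interacting without the key only plays the Keycard_use sound.
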(event EventPickUpKey
  (Variables|Default|SetHas%20Key? true))

(event EventStartInteract
  (params (Player :type Character%20Object%20Reference))
  (if (not (Variables|Default|GetHasInteracted))
    (if (Variables|Default|GetHas%20Key?)
      (bind _outactors (Actor|GetAllActorsOfClass "/Game/TestScenes/Ethan/BP_DoorAnim1.BP_DoorAnim1_C"))
      (bind _array_element (Utilities|Array|ForEachLoopwithBreak _outactors)
        (:LoopBody
          (if (== (Variables|/Game/TestScenes/Ethan/BP_DoorAnim1.BP_DoorAnim1_C|GetDoor%20Value _array_element) (Variables|Default|GetButton%20Value))
            (Default|OpenDoor _array_element (Game|GetPlayerCharacter 0))
            (Game|Player|SetViewTargetwithBlend (Game|GetPlayerController 0) _array_element 0.0 "VTBlend_Linear" 0.0 false)
            (Variables|Default|SetHasInteracted true))))
      (else
        (Audio|PlaySound2D "/Game/Sound_assets/Keycard_use.Keycard_use" 1.0 1.0 0.0 0 0)))))

(fn ConstructionScript)