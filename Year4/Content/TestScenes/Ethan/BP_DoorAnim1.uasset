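; BP_DoorAnim1 is a key-locked door that slides downward when opened, likely a test-scene asset.
; PickUpKey sets HasKey, and OpenDoor only plays the OpenDoorT timeline once that flag is true.
; The timeline lerps DoorAnim's relative location down along Z, then after a short delay blends the first player controller's view target back to the player character.
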(event Custom|Open%20Door
  (params (Player :type Actor%20Object%20Reference))
  (if (Variables|Default|GetHas%20Key?)
    (bind _open_track (Timeline|Open%20Door%20T Play)
      (:Update
        (Transformation|SetRelativeLocation (Variables|Default|GetDoorAnim) (Math|Vector|Lerp(Vector) "0, 0, 0" "0.000000,0.000000,-300.000000" _open_track) false false))
      (:Finished
        (Utilities|FlowControl|Delay 1.0)
        (Game|Player|SetViewTargetwithBlend (Game|GetPlayerController 0) (Game|GetPlayerCharacter 0) 0.0 "VTBlend_Linear" 0.0 false)))))

(event EventPickUpKey
  (Variables|Default|SetHas%20Key? true))

(fn ConstructionScript)