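; Hack station observer that counts hack pickups and relays the running count to walls in the level.
; Hack_Pickup_Event increments the count, prints a debug string and calls AlertWallEvent on every entry in WallArray, passing the count and that wall's array index.
; BeginPlay also caches the first Wall actor found in WallRef, which the pickup logic does not use.
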(event Custom|Hack_Pickup_Event
  (Variables|Default|SetPickup_num (+ (Variables|Default|GetPickup_num) 1))
  (Development|PrintString "pickup")
  (for (_array_element _array_index) (Variables|Default|GetWall_array)
    (Default|AlertWallEvent _array_element (Variables|Default|GetPickup_num) _array_index)))

(event EventBeginPlay
  (bind _outactors (Actor|GetAllActorsOfClass "/Game/Interaction/wall.wall_C"))
  (Variables|Default|SetWall_ref (Utilities|Array|Get(acopy) _outactors)))

(event Collision|EventActorBeginOverlap
  (params (OtherActor :type Actor%20Object%20Reference)))

(event EventTick
  (params (DeltaSeconds :type Float%20%28single-precision%29)))

(fn ConstructionScript)