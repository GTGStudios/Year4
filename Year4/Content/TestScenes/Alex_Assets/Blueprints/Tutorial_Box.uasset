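; Tutorial trigger box that shows an instruction and freezes the game when an overlap begins.
; On BeginPlay it caches the first Tutorial_Manager and third-person character, though the character reference goes unused.
; While ShowText is set, overlap writes the instruction and unpause texts to the manager and zeroes global time dilation, without filtering actors.
; End overlap clears ShowText to make it one-shot, and DisableWidget clears both texts.
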(event OnComponentBeginOverlap(Box)
  (params (OverlappedComponent :type Primitive%20Component%20Object%20Reference) (OtherActor :type Actor%20Object%20Reference) (OtherComp :type Primitive%20Component%20Object%20Reference) (OtherBodyIndex :type Integer) (bFromSweep :type Boolean) (SweepResult :type Hit%20Result%20Structure%20%28by%20ref%29))
  (if (Variables|Default|GetShowText)
    (Variables|/Game/TestScenes/Alex_Assets/Blueprints/Tutorial_Manager.Tutorial_Manager_C|SetTut_Text (Variables|Default|GetManager) (Variables|Default|GetNew_instructions))
    (Variables|/Game/TestScenes/Alex_Assets/Blueprints/Tutorial_Manager.Tutorial_Manager_C|SetUnpauseInst (Variables|Default|GetManager) (Variables|Default|GetPause))
    (Utilities|Time|SetGlobalTimeDilation 0.0)))

(event OnComponentEndOverlap(Box)
  (params (OverlappedComponent :type Primitive%20Component%20Object%20Reference) (OtherActor :type Actor%20Object%20Reference) (OtherComp :type Primitive%20Component%20Object%20Reference) (OtherBodyIndex :type Integer))
  (if (Variables|Default|GetShowText)
    (Variables|Default|SetShowText false)))

(event EventBeginPlay
  (bind _outactors (Actor|GetAllActorsOfClass "/Game/TestScenes/Alex_Assets/Blueprints/Tutorial_Manager.Tutorial_Manager_C"))
  (Variables|Default|SetManager (Utilities|Array|Get(acopy) _outactors))
  (bind _outactors_2 (Actor|GetAllActorsOfClass "/Game/ThirdPerson/Blueprints/BP_ThirdPersonCharacter.BP_ThirdPersonCharacter_C"))
  (Variables|Default|SetCharRef (Utilities|Array|Get(acopy) _outactors_2)))

(event Collision|EventActorBeginOverlap
  (params (OtherActor :type Actor%20Object%20Reference)))

(event EventTick
  (params (DeltaSeconds :type Float%20%28single-precision%29)))

(fn ConstructionScript)

(fn DisableWidget
  (Variables|/Game/TestScenes/Alex_Assets/Blueprints/Tutorial_Manager.Tutorial_Manager_C|SetTut_Text (Variables|Default|GetManager) (Variables|Default|GetInst_clear))
  (Variables|/Game/TestScenes/Alex_Assets/Blueprints/Tutorial_Manager.Tutorial_Manager_C|SetUnpauseInst (Variables|Default|GetManager) (Variables|Default|GetInst_clear)))