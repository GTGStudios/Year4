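; Laser_controls is a test-scene trigger actor that temporarily switches off a set of lasers.
; When anything begins overlapping its Box, it hides every actor in the Laser array and disables their collision, then restores both after a five-second delay.
; It also stores the first BP_IceBullet found in the level on overlap, but never uses it or checks what entered the box.
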(event OnComponentBeginOverlap(Box)
  (params (OverlappedComponent :type Primitive%20Component%20Object%20Reference) (OtherActor :type Actor%20Object%20Reference) (OtherComp :type Primitive%20Component%20Object%20Reference) (OtherBodyIndex :type Integer) (bFromSweep :type Boolean) (SweepResult :type Hit%20Result%20Structure%20%28by%20ref%29))
  (bind _outactors (Actor|GetAllActorsOfClass "/Game/TestScenes/Ethan/BP_IceBullet.BP_IceBullet_C"))
  (Variables|Default|SetIce_bullet (Utilities|Array|Get(acopy) _outactors))
  (for _array_element (Variables|Default|GetLaser)
    (Rendering|SetActorHiddenInGame _array_element true)
    (Collision|SetActorEnableCollision _array_element false))
  (Utilities|FlowControl|Delay 5.0)
  (for _array_element_2 (Variables|Default|GetLaser)
    (Rendering|SetActorHiddenInGame _array_element_2 false)
    (Collision|SetActorEnableCollision _array_element_2 true)))

(event EventBeginPlay)

(event Collision|EventActorBeginOverlap
  (params (OtherActor :type Actor%20Object%20Reference)))

(event EventTick
  (params (DeltaSeconds :type Float%20%28single-precision%29)))

(fn ConstructionScript)