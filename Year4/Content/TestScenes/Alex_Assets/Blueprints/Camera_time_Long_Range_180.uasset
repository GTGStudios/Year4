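; A long-range camera actor that sweeps back and forth in yaw, likely across 180 degrees given its name.
; Tick rotates it at a set speed until its rounded yaw exactly equals the current threshold, then reverses direction and switches to the other threshold.
; An Ice_Block entering its Box pauses the sweep, and leaving resumes it.
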(event OnComponentBeginOverlap(Box)
  (params (OverlappedComponent :type Primitive%20Component%20Object%20Reference) (OtherActor :type Actor%20Object%20Reference) (OtherComp :type Primitive%20Component%20Object%20Reference) (OtherBodyIndex :type Integer) (bFromSweep :type Boolean) (SweepResult :type Hit%20Result%20Structure%20%28by%20ref%29))
  (Utilities|Casting|CastToIce_Block OtherActor)
  (Variables|Default|SetRotate false))

(event OnComponentEndOverlap(Box)
  (params (OverlappedComponent :type Primitive%20Component%20Object%20Reference) (OtherActor :type Actor%20Object%20Reference) (OtherComp :type Primitive%20Component%20Object%20Reference) (OtherBodyIndex :type Integer))
  (Utilities|Casting|CastToIce_Block OtherActor)
  (Variables|Default|SetRotate true))

(event EventBeginPlay
  (|CallParentFunction)
  (Variables|Default|SetChangeThreshold (Variables|Default|GetFirstChangeThreshold)))

(event Collision|EventActorBeginOverlap
  (params (OtherActor :type Actor%20Object%20Reference))
  (|CallParentFunction OtherActor) ; This node is disabled and will not be called.\nDrag off pins to build functionality.
)

(event EventTick
  (params (DeltaSeconds :type Float%20%28single-precision%29))
  (bind _returnvalue (Transformation|GetActorRotation))
  (if (Variables|Default|GetRotate)
    (if (!= (Variables|Default|GetChangeRot) true)
      (if (or (== (Class|KismetMathLibrary|FCeil64 (.yaw _returnvalue)) (Variables|Default|GetChangeThreshold)) (== (Class|KismetMathLibrary|FFloor64 (.yaw _returnvalue)) (Variables|Default|GetChangeThreshold)))
        (Variables|Default|SetChangeRot true)
        (else
          (Transformation|AddActorLocalRotation (Math|Rotator|MakeRotator 0.0 0.0 (* DeltaSeconds (Variables|Default|GetRotation))) false false)))
      (else
        (Variables|Default|SetRotation (* (Variables|Default|GetRotation) -1.0))
        (Variables|Default|SetChangeRot false)
        (if (== (Variables|Default|GetChangeThreshold) (Variables|Default|GetFirstChangeThreshold))
          (Variables|Default|SetChangeThreshold (Variables|Default|GetSecondChamgeThreshold))
          (else
            (Variables|Default|SetChangeThreshold (Variables|Default|GetFirstChangeThreshold))))))))

(fn ConstructionScript
  (|CallParentFunction))