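; A one-shot style trigger actor that removes the main building behind the player and seals the way with a lock door.
; On BeginPlay, the referenced LockDoor is hidden with collision disabled.
; Any overlap of the Box destroys the first found MainBuilding, several DoorEntrance variants and two IndustrialLight lookups through GetActorOfClass, then shows LockDoor and enables its collision.
; Nothing filters the overlapping actor or guards against repeat triggers.
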(event OnComponentBeginOverlap(Box)
  (params (OverlappedComponent :type Primitive%20Component%20Object%20Reference) (OtherActor :type Actor%20Object%20Reference) (OtherComp :type Primitive%20Component%20Object%20Reference) (OtherBodyIndex :type Integer) (bFromSweep :type Boolean) (SweepResult :type Hit%20Result%20Structure%20%28by%20ref%29))
  (bind _lockdoor (Variables|Default|GetLockDoor))
  (bind _returnvalue (Actor|GetActorOfClass "/Game/3D_Assets/World/MainBuilding.MainBuilding_C"))
  (Actor|DestroyActor _returnvalue)
  (bind _returnvalue_2 (Actor|GetActorOfClass "/Game/3D_Assets/architectural_Prefabs/DoorEntrance.DoorEntrance_C"))
  (Actor|DestroyActor _returnvalue_2)
  (bind _returnvalue_3 (Actor|GetActorOfClass "/Game/3D_Assets/architectural_Prefabs/DoorEntrance1.DoorEntrance1_C"))
  (Actor|DestroyActor _returnvalue_3)
  (bind _returnvalue_4 (Actor|GetActorOfClass "/Game/3D_Assets/architectural_Prefabs/DoorEntrance2.DoorEntrance2_C"))
  (Actor|DestroyActor _returnvalue_4)
  (bind _returnvalue_5 (Actor|GetActorOfClass "/Game/3D_Assets/Reidslights/IndustrialLight/IndustrialLight.IndustrialLight_C"))
  (Actor|DestroyActor _returnvalue_5)
  (bind _returnvalue_6 (Actor|GetActorOfClass "/Game/3D_Assets/Reidslights/IndustrialLight/IndustrialLight.IndustrialLight_C"))
  (Actor|DestroyActor _returnvalue_6)
  (bind _returnvalue_7 (Actor|GetActorOfClass "/Game/3D_Assets/architectural_Prefabs/DoorEntrance3.DoorEntrance3_C"))
  (Actor|DestroyActor _returnvalue_7)
  (Rendering|SetActorHiddenInGame _lockdoor false)
  (Collision|SetActorEnableCollision _lockdoor true))

(event EventBeginPlay
  (bind _lockdoor (Variables|Default|GetLockDoor))
  (Rendering|SetActorHiddenInGame _lockdoor true)
  (Collision|SetActorEnableCollision _lockdoor false))

(event EventTick
  (params (DeltaSeconds :type Float%20%28single-precision%29)))

(fn ConstructionScript)