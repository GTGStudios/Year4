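; BP_Circuit draws a circuit of line actors between consecutive points in PointList and supports swapping two points.
; UpdateCircuit, run on BeginPlay, destroys the actors in LineList, then spawns a BP_CircutLine at each segment's midpoint.
; Each line is rotated along the segment direction and scaled to its length, minus a fixed gap.
; SwapDuo exchanges the locations of the two SwappingDuo actors, rebuilds the lines and clears the pair.
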(event Custom|update%20circuit
  (bind _pointlist (Variables|Default|GetPointList))
  (for _array_element (Variables|Default|GetLineList)
    (Actor|DestroyActor _array_element))
  (for (_ _array_index) _pointlist
    (if (not (== _array_index 0))
      (bind _returnvalue (Game|SpawnActorfromClass "/Game/Blueprints/BP_CircutLine.BP_CircutLine_C" (Math|Conversions|ToTransform(Vector) (+ (/ (- (Transformation|GetActorLocation (Utilities|Array|Get(acopy) _pointlist _array_index)) (Transformation|GetActorLocation (Utilities|Array|Get(acopy) _pointlist (- _array_index 1)))) "2.000000,2.000000,2.000000") (Transformation|GetActorLocation (Utilities|Array|Get(acopy) _pointlist (- _array_index 1))))) "Undefined" "OverrideRootScale" 0 0))
      (Transformation|SetActorRotation _returnvalue (Math|Conversions|RotationFromXVector (Math|Vector|MakeVector (/ (.X (Math|Vector|BreakVector (- (Transformation|GetActorLocation (Utilities|Array|Get(acopy) _pointlist _array_index)) (Transformation|GetActorLocation (Utilities|Array|Get(acopy) _pointlist (- _array_index 1)))))) (Math|Float|Sqrt (+ (Math|Float|Square (.X (Math|Vector|BreakVector (- (Transformation|GetActorLocation (Utilities|Array|Get(acopy) _pointlist _array_index)) (Transformation|GetActorLocation (Utilities|Array|Get(acopy) _pointlist (- _array_index 1))))))) (Math|Float|Square (.Y (Math|Vector|BreakVector (- (Transformation|GetActorLocation (Utilities|Array|Get(acopy) _pointlist _array_index)) (Transformation|GetActorLocation (Utilities|Array|Get(acopy) _pointlist (- _array_index 1))))))) (Math|Float|Square (.Z (Math|Vector|BreakVector (- (Transformation|GetActorLocation (Utilities|Array|Get(acopy) _pointlist _array_index)) (Transformation|GetActorLocation (Utilities|Array|Get(acopy) _pointlist (- _array_index 1)))))))))) (/ (.Y (Math|Vector|BreakVector (- (Transformation|GetActorLocation (Utilities|Array|Get(acopy) _pointlist _array_index)) (Transformation|GetActorLocation (Utilities|Array|Get(acopy) _pointlist (- _array_index 1)))))) (Math|Float|Sqrt (+ (Math|Float|Square (.X (Math|Vector|BreakVector (- (Transformation|GetActorLocation (Utilities|Array|Get(acopy) _pointlist _array_index)) (Transformation|GetActorLocation (Utilities|Array|Get(acopy) _pointlist (- _array_index 1))))))) (Math|Float|Square (.Y (Math|Vector|BreakVector (- (Transformation|GetActorLocation (Utilities|Array|Get(acopy) _pointlist _array_index)) (Transformation|GetActorLocation (Utilities|Array|Get(acopy) _pointlist (- _array_index 1))))))) (Math|Float|Square (.Z (Math|Vector|BreakVector (- (Transformation|GetActorLocation (Utilities|Array|Get(acopy) _pointlist _array_index)) (Transformation|GetActorLocation (Utilities|Array|Get(acopy) _pointlist (- _array_index 1)))))))))) (/ (.Z (Math|Vector|BreakVector (- (Transformation|GetActorLocation (Utilities|Array|Get(acopy) _pointlist _array_index)) (Transformation|GetActorLocation (Utilities|Array|Get(acopy) _pointlist (- _array_index 1)))))) (Math|Float|Sqrt (+ (Math|Float|Square (.X (Math|Vector|BreakVector (- (Transformation|GetActorLocation (Utilities|Array|Get(acopy) _pointlist _array_index)) (Transformation|GetActorLocation (Utilities|Array|Get(acopy) _pointlist (- _array_index 1))))))) (Math|Float|Square (.Y (Math|Vector|BreakVector (- (Transformation|GetActorLocation (Utilities|Array|Get(acopy) _pointlist _array_index)) (Transformation|GetActorLocation (Utilities|Array|Get(acopy) _pointlist (- _array_index 1))))))) (Math|Float|Square (.Z (Math|Vector|BreakVector (- (Transformation|GetActorLocation (Utilities|Array|Get(acopy) _pointlist _array_index)) (Transformation|GetActorLocation (Utilities|Array|Get(acopy) _pointlist (- _array_index 1)))))))))))))
      (Transformation|SetActorScale3D _returnvalue (* (Math|Vector|MakeVector (- (Math|Float|Sqrt (+ (Math|Float|Square (.X (Math|Vector|BreakVector (- (Transformation|GetActorLocation (Utilities|Array|Get(acopy) _pointlist _array_index)) (Transformation|GetActorLocation (Utilities|Array|Get(acopy) _pointlist (- _array_index 1))))))) (Math|Float|Square (.Y (Math|Vector|BreakVector (- (Transformation|GetActorLocation (Utilities|Array|Get(acopy) _pointlist _array_index)) (Transformation|GetActorLocation (Utilities|Array|Get(acopy) _pointlist (- _array_index 1))))))) (Math|Float|Square (.Z (Math|Vector|BreakVector (- (Transformation|GetActorLocation (Utilities|Array|Get(acopy) _pointlist _array_index)) (Transformation|GetActorLocation (Utilities|Array|Get(acopy) _pointlist (- _array_index 1))))))))) 4e+01) 1e+01 1e+01) "0.010000,0.100000,0.100000"))
      (Utilities|Array|Add (Variables|Default|GetLineList) _returnvalue))))

(event Custom|SwapDuo
  (bind _swappingduo (Variables|Default|GetswappingDuo))
  (bind _output (Utilities|Array|Get(acopy) _swappingduo))
  (bind _output_2 (Utilities|Array|Get(acopy) _swappingduo 1))
  (bind _output_get (Variables|Default|Setswappingduo1vector (Transformation|GetActorLocation _output)))
  (Transformation|SetActorLocation _output (Transformation|GetActorLocation _output_2) false false)
  (Transformation|SetActorLocation _output_2 _output_get false false)
  (CallFunction|UpdateCircuit)
  (Utilities|Array|Clear (Variables|Default|GetswappingDuo)))

(event EventBeginPlay
  (CallFunction|UpdateCircuit))

(event Collision|EventActorBeginOverlap
  (params (OtherActor :type Actor%20Object%20Reference)))

(event EventTick
  (params (DeltaSeconds :type Float%20%28single-precision%29)))

(fn ConstructionScript)