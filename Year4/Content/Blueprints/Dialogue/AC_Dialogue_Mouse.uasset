(fn Dialogue
  (|CallParentFunction)
  (switch int (Variables|Default|GetDialogueTreeIndex)
    (:0
      (bind (_state _optionindex) (CallFunction|AddDialogue "Mouse" "Hi how are you" (Utilities|Array|MakeArray "Good" "Bad")))
      (switch Utilities|FlowControl|Switch|SwitchonEnum_DialogueState _state
        (:NewEnumerator0
          (switch int _optionindex
            (:0
              (bind (_state_2 _optionindex_2) (CallFunction|AddDialogue "Mouse" "Wonderful, can I have $250?" (Utilities|Array|MakeArray "Give Money" "Keep Money")))
              (switch Utilities|FlowControl|Switch|SwitchonEnum_DialogueState _state_2
                (:NewEnumerator0
                  (switch int _optionindex_2
                    (:0
                      (bind _state_3 (CallFunction|AddDialogue "Mouse" "Thank You" (Utilities|Array|MakeArray "Continue")))
                      (switch Utilities|FlowControl|Switch|SwitchonEnum_DialogueState _state_3
                        (:NewEnumerator0
                          (CallFunction|SetDialogueTreeIndex 1)
                          (CallFunction|CloseConversation))))
                    (:1
                      (bind _state_4 (CallFunction|AddDialogue "Mouse" "How Rude" (Utilities|Array|MakeArray "Continue")))
                      (switch Utilities|FlowControl|Switch|SwitchonEnum_DialogueState _state_4
                        (:NewEnumerator0
                          (CallFunction|RemoveDialogueProgress 2)
                          (CallFunction|CloseConversation))))))))
            (:1
              (bind _state_5 (CallFunction|AddDialogue "Mouse" "Oh that's a shame." (Utilities|Array|MakeArray "Continue")))
              (switch Utilities|FlowControl|Switch|SwitchonEnum_DialogueState _state_5
                (:NewEnumerator0
                  (CallFunction|ClearDialogueProgress)
                  (CallFunction|CloseConversation))))))))
    (:1
      (bind _state_6 (CallFunction|AddDialogue "Mouse" "Thanks for the money!!" (Utilities|Array|MakeArray "Continue")))
      (switch Utilities|FlowControl|Switch|SwitchonEnum_DialogueState _state_6
        (:NewEnumerator0
          (CallFunction|ClearDialogueProgress)
          (CallFunction|CloseConversation))))))