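; AC_Dialogue_Bot is a dialogue component for the Bot, which offers a stuck player a hint about raising a white platform.
; It overrides Dialogue, calls the parent, then switches on DialogueTreeIndex, branching AddDialogue lines on state and chosen option.
; Accepting help advances the tree to a "Goodluck!" line, while declining or finishing that line clears progress, and each path closes the conversation.
; An unconnected branch holds unused Bot and Mouse lines.
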(fn Dialogue
  (|CallParentFunction)
  (switch int (Variables|Default|GetDialogueTreeIndex)
    (:0
      (bind (_state _optionindex) (CallFunction|AddDialogue "Bot" "Hi are you stuck?" (Utilities|Array|MakeArray "Yes, help!" "No, I know what I'm doing") "/Game/Sound_assets/Dialogue/DialogueRobot2.DialogueRobot2"))
      (switch Utilities|FlowControl|Switch|SwitchonEnum_DialogueState _state
        (:NewEnumerator0
          (switch int _optionindex
            (:0
              (bind _state_2 (CallFunction|AddDialogue "Bot" "There is a white platform on the ground over there, you should be able to interact with it to raise it up." (Utilities|Array|MakeArray "Continue")))
              (switch Utilities|FlowControl|Switch|SwitchonEnum_DialogueState _state_2
                (:NewEnumerator0
                  (CallFunction|SetDialogueTreeIndex 1)
                  (CallFunction|CloseConversation))))
            (:1
              (bind _state_3 (CallFunction|AddDialogue "Bot" "Great! Be careful out there." (Utilities|Array|MakeArray "Continue")))
              (switch Utilities|FlowControl|Switch|SwitchonEnum_DialogueState _state_3
                (:NewEnumerator0
                  (CallFunction|ClearDialogueProgress)
                  (CallFunction|CloseConversation))))))))
    (:1
      (bind _state_4 (CallFunction|AddDialogue "Bot" "Goodluck!" (Utilities|Array|MakeArray "Continue")))
      (switch Utilities|FlowControl|Switch|SwitchonEnum_DialogueState _state_4
        (:NewEnumerator0
          (CallFunction|ClearDialogueProgress)
          (CallFunction|CloseConversation))))))