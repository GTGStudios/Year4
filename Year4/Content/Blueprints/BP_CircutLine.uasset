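; BP_CircutLine is a circuit line actor with a Cube component, apparently an unfinished piece of a circuit system.
; On BeginPlay it caches the first BP_Circuit actor it finds.
; Every Tick it checks each LineList entry of that circuit against the Cube's overlapping actors, but a match triggers nothing yet.
; A hit on the Cube prints the line's own name, while the overlap events are empty.
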(event OnComponentBeginOverlap(Cube)
  (params (OverlappedComponent :type Primitive%20Component%20Object%20Reference) (OtherActor :type Actor%20Object%20Reference) (OtherComp :type Primitive%20Component%20Object%20Reference) (OtherBodyIndex :type Integer) (bFromSweep :type Boolean) (SweepResult :type Hit%20Result%20Structure%20%28by%20ref%29)))

(event OnComponentHit(Cube)
  (params (HitComponent :type Primitive%20Component%20Object%20Reference) (OtherActor :type Actor%20Object%20Reference) (OtherComp :type Primitive%20Component%20Object%20Reference) (NormalImpulse :type Vector :default "0, 0, 0") (Hit :type Hit%20Result%20Structure%20%28by%20ref%29))
  (Development|PrintString (Utilities|GetDisplayName self)))

(event EventBeginPlay
  (bind _returnvalue (Actor|GetActorOfClass "/Game/Blueprints/BP_Circuit.BP_Circuit_C"))
  (Variables|Default|SetCircuitRef _returnvalue))

(event Collision|EventActorBeginOverlap
  (params (OtherActor :type Actor%20Object%20Reference)))

(event EventTick
  (params (DeltaSeconds :type Float%20%28single-precision%29))
  (for _array_element (Variables|/Game/Blueprints/BP_Circuit.BP_Circuit_C|GetLineList (Variables|Default|GetCircuitRef))
    (if (Utilities|Array|ContainsItem (Collision|GetOverlappingActors (Variables|Default|GetCube) 0 :!class /Script/Engine.PrimitiveComponent) _array_element)
      _)))

(fn ConstructionScript)