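; BP_CCTV1 is a security camera actor that blinds the screen while something tagged Detectable is inside its detection cone.
; Cone overlaps set and clear a Detected flag, with entry ignored when Frozen.
; While Detected, every Tick creates a new WBP_BlindEffect widget, adds it to the viewport and calls its Fading.
; Hits from freezingBullet-tagged actors only print a message; nothing here sets Frozen.
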(event OnComponentBeginOverlap(Cone)
  (params (OverlappedComponent :type Primitive%20Component%20Object%20Reference) (OtherActor :type Actor%20Object%20Reference) (OtherComp :type Primitive%20Component%20Object%20Reference) (OtherBodyIndex :type Integer) (bFromSweep :type Boolean) (SweepResult :type Hit%20Result%20Structure%20%28by%20ref%29))
  (if (Actor|ActorHasTag OtherActor "Detectable")
    (if (not (Variables|Default|GetFrozen))
      (Development|PrintString "Detected2")
      (Variables|Default|SetDetected true))))

(event OnComponentEndOverlap(Cone)
  (params (OverlappedComponent :type Primitive%20Component%20Object%20Reference) (OtherActor :type Actor%20Object%20Reference) (OtherComp :type Primitive%20Component%20Object%20Reference) (OtherBodyIndex :type Integer))
  (if (Actor|ActorHasTag OtherActor "Detectable")
    (Development|PrintString "exiting2")
    (Variables|Default|SetDetected false)))

(event OnComponentHit(StaticMesh)
  (params (HitComponent :type Primitive%20Component%20Object%20Reference) (OtherActor :type Actor%20Object%20Reference) (OtherComp :type Primitive%20Component%20Object%20Reference) (NormalImpulse :type Vector :default "0, 0, 0") (Hit :type Hit%20Result%20Structure%20%28by%20ref%29))
  (if (Actor|ActorHasTag OtherActor "freezingBullet")
    (Development|PrintString "CCTVFrozen")))

(event EventBeginPlay
  (bind _asbp_third_person_character (Utilities|Casting|CastToBP_ThirdPersonCharacter (Game|GetPlayerCharacter 0)))
  (Variables|Default|SetPlayer _asbp_third_person_character))

(event Collision|EventActorBeginOverlap
  (params (OtherActor :type Actor%20Object%20Reference)))

(event EventTick
  (params (DeltaSeconds :type Float%20%28single-precision%29))
  (if (Variables|Default|GetDetected)
    (bind _returnvalue (UserInterface|CreateWidget "/Game/Blueprints/WBP_BlindEffect.WBP_BlindEffect_C"))
    (UserInterface|Viewport|AddtoViewport _returnvalue 0)
    (Default|Fading _returnvalue)))

(fn ConstructionScript)