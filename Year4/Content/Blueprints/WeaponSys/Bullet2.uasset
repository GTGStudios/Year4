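; Bullet2 is a physics projectile that spawns an Ice_Block where it hits and then destroys itself.
; On BeginPlay its Sphere receives a fixed impulse in world X and Y, independent of the actor's rotation.
; The Sphere's hit event handles the spawn, a debug print and the destroy.
; A separate actor Hit event pushes physics-simulating components with an impulse scaled from the bullet's velocity.
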(event OnComponentHit(Sphere)
  (params (HitComponent :type Primitive%20Component%20Object%20Reference) (OtherActor :type Actor%20Object%20Reference) (OtherComp :type Primitive%20Component%20Object%20Reference) (NormalImpulse :type Vector :default "0, 0, 0") (Hit :type Hit%20Result%20Structure%20%28by%20ref%29))
  (Game|SpawnActorfromClass "/Game/TestScenes/Alex_Assets/Ice_Block.Ice_Block_C" (Math|Conversions|ToTransform(Vector) (Transformation|GetWorldLocation (Variables|Default|GetSphere))) "Undefined" "MultiplyWithRoot" 0 0)
  (Development|PrintString "hit")
  (Actor|DestroyActor))

(event EventBeginPlay
  (Physics|AddImpulse (Variables|Default|GetSphere) "100.000000,100.000000,0.000000" "None" false))

(event Collision|EventActorBeginOverlap
  (params (OtherActor :type Actor%20Object%20Reference)))

(event EventTick
  (params (DeltaSeconds :type Float%20%28single-precision%29)))

(event Collision|EventHit
  (params (MyComp :type Primitive%20Component%20Object%20Reference) (Other :type Actor%20Object%20Reference) (OtherComp :type Primitive%20Component%20Object%20Reference) (bSelfMoved :type Boolean) (HitLocation :type Vector :default "0, 0, 0") (HitNormal :type Vector :default "0, 0, 0") (NormalImpulse :type Vector :default "0, 0, 0") (Hit :type Hit%20Result%20Structure%20%28by%20ref%29))
  (if (Physics|IsSimulatingPhysics OtherComp "None")
    (Physics|AddImpulseatLocation OtherComp (* (Transformation|GetVelocity) 5e+02) (Transformation|GetActorLocation) "None")))

(fn ConstructionScript)