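; Interactable key pickup that notifies its linked door and switches on a set of cameras, with no cutscene.
; On BeginPlay it disables each listed camera's rotation, activation and spotlight.
; Interacting triggers the door's pickup message, swaps in a dissolve material, then destroys the key after a zero-length delay and re-enables those cameras at high light intensity.
; Tick advances the dissolve's Progress parameter, though the immediate destroy leaves it little time to show.
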(event EventBeginPlay
  (bind _cameraactivationlist (Variables|Default|GetCameraActivationList))
  (if (> (Utilities|Array|Length _cameraactivationlist) 0)
    (for _array_element _cameraactivationlist
      (Variables|/Game/Blueprints/Alex_Assets/Blueprints/Camera_time_Long_Range_180.Camera_time_Long_Range_180_C|SetRotate _array_element false)
      (Variables|/Game/Blueprints/Alex_Assets/Blueprints/Camera_time_Long_Range.Camera_time_Long_Range_C|SetActivated _array_element false)
      (Rendering|Components|Light|SetIntensity (Variables|/Game/Blueprints/Alex_Assets/Blueprints/Camera_time_Long_Range.Camera_time_Long_Range_C|GetSpotLight _array_element) 0.0))))

(event Collision|EventActorBeginOverlap
  (params (OtherActor :type Actor%20Object%20Reference)))

(event EventTick
  (params (DeltaSeconds :type Float%20%28single-precision%29))
  (if (Variables|Default|GetDissolve)
    (Utilities|FlowControl|Delay 0.05)
    (bind _output_get (Variables|Default|SetProgress (+ (Variables|Default|GetProgress) 0.01)))
    (Rendering|Material|SetScalarParameterValueonMaterials (Variables|Default|GetSphere) "Progress" _output_get)))

(event EventStartInteract
  (params (Player :type Character%20Object%20Reference))
  (Class|BPIDoor|PickUpKey(Message) (Variables|Default|GetDoorNoCutscene))
  (Rendering|Material|SetMaterial (Variables|Default|GetSphere) 0 "/Game/Blueprints/Alex_Assets/Materials/Dissolve_Inst.Dissolve_Inst")
  (Variables|Default|SetDissolve true)
  (Utilities|FlowControl|Delay 0.0)
  (Variables|Default|SetDissolve false)
  (Actor|DestroyActor)
  (if (> (Utilities|Array|Length (Variables|Default|GetCameraActivationList)) 0)
    (for _array_element (Variables|Default|GetCameraActivationList)
      (Variables|/Game/Blueprints/Alex_Assets/Blueprints/Camera_time_Long_Range.Camera_time_Long_Range_C|SetActivated _array_element true)
      (Variables|/Game/Blueprints/Alex_Assets/Blueprints/Camera_time_Long_Range_180.Camera_time_Long_Range_180_C|SetRotate _array_element true)
      (Rendering|Components|Light|SetIntensity (Variables|/Game/Blueprints/Alex_Assets/Blueprints/Camera_time_Long_Range.Camera_time_Long_Range_C|GetSpotLight _array_element) 1e+05))))

(fn ConstructionScript)

(fn ChangeProgressMaterial)