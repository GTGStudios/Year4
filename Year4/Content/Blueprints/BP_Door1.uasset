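; BP_Door1 is a keyed door that slides downward to open when interacted with once the key is picked up.
; StartInteract checks HasKey, then a FlipFlop alternately plays and reverses a Timeline that lerps the Door's relative location.
; Without the key, it shows a temporary DoorLockedText widget and plays a keycard sound.
; PickUpKey sets HasKey to unlock it.
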(event EventBeginPlay)

(event EventTick
  (params (DeltaSeconds :type Float%20%28single-precision%29)))

(event Collision|EventActorBeginOverlap
  (params (OtherActor :type Actor%20Object%20Reference)))

(event EventStartInteract
  (if (Variables|Default|GetHas%20Key?)
    (Utilities|FlowControl|FlipFlop
      (:A
        (bind _open_door_1 (Timeline|Timeline Play)
          (:Update
            (Transformation|SetRelativeLocation (Variables|Default|GetDoor) (Math|Vector|Lerp(Vector) "0, 0, 0" "0.000000,0.000000,-310.000000" _open_door_1) false false))))
      (:B
        (Timeline|Timeline Reverse)))
    (else
      (bind _returnvalue (UserInterface|CreateWidget "/Game/Blueprints/DoorLockedText.DoorLockedText_C"))
      (UserInterface|Viewport|AddtoViewport _returnvalue 0)
      (Audio|PlaySound2D "/Game/Sound_assets/Keycard_use.Keycard_use" 1.0 1.0 0.0 0 0)
      (Utilities|FlowControl|Delay 4.0)
      (Widget|RemovefromParent _returnvalue))))

(event EventPickUpKey
  (Variables|Default|SetHas%20Key? true))

(fn ConstructionScript)