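; Circuit puzzle manager that activates a teleporter and destroys DeleteList actors once every connecting line is working.
; Each update rebuilds the BP_CircutLine actors between consecutive PointList actors, oriented and stretched to fit, and runs their collision checks.
; SwapDuo exchanges two selected points' positions, resets their materials and triggers an update.
; BeginPlay runs the first update before caching the first Deactivated_tp found in the level.
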(event Custom|update%20circuit
  (bind _pointlist (Variables|Default|GetPointList))
  (bind _linelist (Variables|Default|GetLineList))
  (bind _linelist_2 (Variables|Default|GetLineList))
  (if (Utilities|Array|IsNotEmpty _linelist_2)
    (for _array_element _linelist_2
      (Actor|DestroyActor _array_element))
    (Utilities|Array|Clear _linelist_2))
  (for (_ _array_index) _pointlist
    (if (not (== _array_index 0))
      (bind _returnvalue (Game|SpawnActorfromClass "/Game/Blueprints/CircuitPuzzle/BP_CircutLine.BP_CircutLine_C" (Math|Conversions|ToTransform(Vector) (+ (/ (- (Transformation|GetActorLocation (Utilities|Array|Get(acopy) _pointlist _array_index)) (Transformation|GetActorLocation (Utilities|Array|Get(acopy) _pointlist (- _array_index 1)))) "2.000000,2.000000,2.000000") (Transformation|GetActorLocation (Utilities|Array|Get(acopy) _pointlist (- _array_index 1))))) "Undefined" "OverrideRootScale" 0 0))
      (Transformation|SetActorRotation _returnvalue (Math|Conversions|RotationFromXVector (Math|Vector|MakeVector (/ (.X (Math|Vector|BreakVector (- (Transformation|GetActorLocation (Utilities|Array|Get(acopy) _pointlist _array_index)) (Transformation|GetActorLocation (Utilities|Array|Get(acopy) _pointlist (- _array_index 1)))))) (Math|Float|Sqrt (+ (Math|Float|Square (.X (Math|Vector|BreakVector (- (Transformation|GetActorLocation (Utilities|Array|Get(acopy) _pointlist _array_index)) (Transformation|GetActorLocation (Utilities|Array|Get(acopy) _pointlist (- _array_index 1))))))) (Math|Float|Square (.Y (Math|Vector|BreakVector (- (Transformation|GetActorLocation (Utilities|Array|Get(acopy) _pointlist _array_index)) (Transformation|GetActorLocation (Utilities|Array|Get(acopy) _pointlist (- _array_index 1))))))) (Math|Float|Square (.Z (Math|Vector|BreakVector (- (Transformation|GetActorLocation (Utilities|Array|Get(acopy) _pointlist _array_index)) (Transformation|GetActorLocation (Utilities|Array|Get(acopy) _pointlist (- _array_index 1)))))))))) (/ (.Y (Math|Vector|BreakVector (- (Transformation|GetActorLocation (Utilities|Array|Get(acopy) _pointlist _array_index)) (Transformation|GetActorLocation (Utilities|Array|Get(acopy) _pointlist (- _array_index 1)))))) (Math|Float|Sqrt (+ (Math|Float|Square (.X (Math|Vector|BreakVector (- (Transformation|GetActorLocation (Utilities|Array|Get(acopy) _pointlist _array_index)) (Transformation|GetActorLocation (Utilities|Array|Get(acopy) _pointlist (- _array_index 1))))))) (Math|Float|Square (.Y (Math|Vector|BreakVector (- (Transformation|GetActorLocation (Utilities|Array|Get(acopy) _pointlist _array_index)) (Transformation|GetActorLocation (Utilities|Array|Get(acopy) _pointlist (- _array_index 1))))))) (Math|Float|Square (.Z (Math|Vector|BreakVector (- (Transformation|GetActorLocation (Utilities|Array|Get(acopy) _pointlist _array_index)) (Transformation|GetActorLocation (Utilities|Array|Get(acopy) _pointlist (- _array_index 1)))))))))) (/ (.Z (Math|Vector|BreakVector (- (Transformation|GetActorLocation (Utilities|Array|Get(acopy) _pointlist _array_index)) (Transformation|GetActorLocation (Utilities|Array|Get(acopy) _pointlist (- _array_index 1)))))) (Math|Float|Sqrt (+ (Math|Float|Square (.X (Math|Vector|BreakVector (- (Transformation|GetActorLocation (Utilities|Array|Get(acopy) _pointlist _array_index)) (Transformation|GetActorLocation (Utilities|Array|Get(acopy) _pointlist (- _array_index 1))))))) (Math|Float|Square (.Y (Math|Vector|BreakVector (- (Transformation|GetActorLocation (Utilities|Array|Get(acopy) _pointlist _array_index)) (Transformation|GetActorLocation (Utilities|Array|Get(acopy) _pointlist (- _array_index 1))))))) (Math|Float|Square (.Z (Math|Vector|BreakVector (- (Transformation|GetActorLocation (Utilities|Array|Get(acopy) _pointlist _array_index)) (Transformation|GetActorLocation (Utilities|Array|Get(acopy) _pointlist (- _array_index 1)))))))))))))
      (Transformation|SetActorScale3D _returnvalue (* (Math|Vector|MakeVector (- (Math|Float|Sqrt (+ (Math|Float|Square (.X (Math|Vector|BreakVector (- (Transformation|GetActorLocation (Utilities|Array|Get(acopy) _pointlist _array_index)) (Transformation|GetActorLocation (Utilities|Array|Get(acopy) _pointlist (- _array_index 1))))))) (Math|Float|Square (.Y (Math|Vector|BreakVector (- (Transformation|GetActorLocation (Utilities|Array|Get(acopy) _pointlist _array_index)) (Transformation|GetActorLocation (Utilities|Array|Get(acopy) _pointlist (- _array_index 1))))))) (Math|Float|Square (.Z (Math|Vector|BreakVector (- (Transformation|GetActorLocation (Utilities|Array|Get(acopy) _pointlist _array_index)) (Transformation|GetActorLocation (Utilities|Array|Get(acopy) _pointlist (- _array_index 1))))))))) 6e+01) 8.0 8.0) "0.010000,0.100000,0.100000"))
      (Utilities|Array|Add _linelist _returnvalue)
      (for _array_element_2 _linelist
        (Default|CheckifColliding _array_element_2))))
  (Variables|Default|SetLoopA1keepGoing true)
  (bind _array_element_3 (Utilities|Array|ForEachLoopwithBreak (Variables|Default|GetLineList))
    (:LoopBody
      (if (Variables|Default|GetLoopA1keepGoing)
        (if (not (Variables|/Game/Blueprints/CircuitPuzzle/BP_CircutLine.BP_CircutLine_C|GetIsWorking _array_element_3))
          (Variables|Default|SetLoopA1keepGoing false))))
    (:Completed
      (if (Variables|Default|GetLoopA1keepGoing)
        (Default|ActivateTp (Variables|Default|GetDeactivated_tp))
        (if (Utilities|Array|IsNotEmpty (Variables|Default|GetDelete%20list))
          (for _array_element_4 (Variables|Default|GetDelete%20list)
            (Actor|DestroyActor _array_element_4)))))))

(event Custom|SwapDuo
  (bind _swappingduo (Variables|Default|GetswappingDuo))
  (bind _output (Utilities|Array|Get(acopy) _swappingduo))
  (bind _output_2 (Utilities|Array|Get(acopy) _swappingduo 1))
  (bind _output_get (Variables|Default|Setswappingduo1vector (Transformation|GetActorLocation _output)))
  (Transformation|SetActorLocation _output (Transformation|GetActorLocation _output_2) false false)
  (Default|Todefaultmaterial _output)
  (Transformation|SetActorLocation _output_2 _output_get false false)
  (Default|Todefaultmaterial _output_2)
  (CallFunction|UpdateCircuit)
  (Utilities|Array|Clear (Variables|Default|GetswappingDuo)))

(event EventBeginPlay
  (CallFunction|UpdateCircuit)
  (bind _outactors (Actor|GetAllActorsOfClass "/Game/Blueprints/Alex_Assets/Blueprints/Deactivated_tp.Deactivated_tp_C"))
  (Variables|Default|SetDeactivated_tp (Utilities|Array|Get(acopy) _outactors)))

(event Collision|EventActorBeginOverlap
  (params (OtherActor :type Actor%20Object%20Reference)))

(event EventTick
  (params (DeltaSeconds :type Float%20%28single-precision%29)))

(fn ConstructionScript)