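; Selectable point in the circuit puzzle that the player interacts with to pick pairs for swapping.
; On BeginPlay it finds the BP_Circuit actor in the level and applies its default material.
; StartInteract highlights the cube, prints its name and adds itself uniquely to the circuit's SwappingDuo array, calling SwapDuo once two are selected.
; A separate event restores the default material.
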(event Custom|todefaultmaterial
  (Rendering|Material|SetMaterial (Variables|Default|GetCube) 0 (Variables|Default|Getdefaultmaterial)))

(event EventBeginPlay
  (bind _returnvalue (Actor|GetActorOfClass "/Game/Blueprints/CircuitPuzzle/BP_Circuit.BP_Circuit_C"))
  (Variables|Default|SetCircuit _returnvalue)
  (CallFunction|Todefaultmaterial))

(event Collision|EventActorBeginOverlap
  (params (OtherActor :type Actor%20Object%20Reference)))

(event EventTick
  (params (DeltaSeconds :type Float%20%28single-precision%29)))

(event EventStartInteract
  (params (Player :type Character%20Object%20Reference))
  (bind _circuit (Variables|Default|GetCircuit))
  (bind _swappingduo (Variables|/Game/Blueprints/CircuitPuzzle/BP_Circuit.BP_Circuit_C|GetswappingDuo _circuit))
  (Rendering|Material|SetMaterial (Variables|Default|GetCube) 0 "/Game/Blueprints/CircuitPuzzle/gram7.gram7")
  (Development|PrintString (Utilities|GetDisplayName self))
  (Utilities|Array|AddUnique _swappingduo self)
  (if (== (Utilities|Array|Length _swappingduo) 2)
    (Default|SwapDuo _circuit)))

(fn ConstructionScript)