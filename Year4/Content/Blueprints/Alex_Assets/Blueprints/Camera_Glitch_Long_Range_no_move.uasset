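; Rotating long-range security camera that detects pawns with PawnSensing and "hacks" the player.
; On sight it enables the Glitch_Process post-process volume, plays an alert, calls HackedMove on either third-person character type and sets IsDetected, readable through GetIsDetected.
; A retriggerable five-second delay clears the glitch and detection flag.
; An Ice_Block overlapping its Box pauses the rotation until it leaves.
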(event OnSeePawn(PawnSensing)
  (params (Pawn :type Pawn%20Object%20Reference))
  (Utilities|FlowControl|Sequence
    (:then_0
      (Variables|/Script/Engine.PostProcessVolume|SetbEnabled (Variables|Default|GetGlitch_Post_Process_Volume) true)
      (Development|PrintString "You are being hacked")
      (Variables|Default|SetIsDetected true)
      (Audio|PlaySound2D "/Game/Blueprints/Alex_Assets/Sounds/alert_mk1.alert_mk1" 1.0 1.0 0.0 0 0)
      (bind _asbp_third_person_character (Utilities|Casting|CastToBP_ThirdPersonCharacter Pawn)
        (:then
          (Default|HackedMove _asbp_third_person_character))
        (:CastFailed
          (bind _asbp_third_person_character_2 (Utilities|Casting|CastToBP_ThirdPersonCharacter2 Pawn)
            (:then
              (Default|HackedMove _asbp_third_person_character_2))
            (:CastFailed
              (Development|PrintString "Fail_CameraGlitch1"))))))
    (:then_1
      (Utilities|FlowControl|RetriggerableDelay 5.0)
      (Variables|/Script/Engine.PostProcessVolume|SetbEnabled (Variables|Default|GetGlitch_Post_Process_Volume) false)
      (Variables|Default|SetIsDetected false))))

(event OnComponentBeginOverlap(Box)
  (params (OverlappedComponent :type Primitive%20Component%20Object%20Reference) (OtherActor :type Actor%20Object%20Reference) (OtherComp :type Primitive%20Component%20Object%20Reference) (OtherBodyIndex :type Integer) (bFromSweep :type Boolean) (SweepResult :type Hit%20Result%20Structure%20%28by%20ref%29))
  (Utilities|Casting|CastToIce_Block OtherActor)
  (Components|Activation|Deactivate (Variables|Default|GetRotatingMovement)))

(event OnComponentEndOverlap(Box)
  (params (OverlappedComponent :type Primitive%20Component%20Object%20Reference) (OtherActor :type Actor%20Object%20Reference) (OtherComp :type Primitive%20Component%20Object%20Reference) (OtherBodyIndex :type Integer))
  (Utilities|Casting|CastToIce_Block OtherActor)
  (Components|Activation|Activate (Variables|Default|GetRotatingMovement) false))

(event EventBeginPlay
  (|CallParentFunction) ; This node is disabled and will not be called.\nDrag off pins to build functionality.
)

(event Collision|EventActorBeginOverlap
  (params (OtherActor :type Actor%20Object%20Reference))
  (|CallParentFunction OtherActor) ; This node is disabled and will not be called.\nDrag off pins to build functionality.
)

(event EventTick
  (params (DeltaSeconds :type Float%20%28single-precision%29)))

(event EventBeginPlay
  (bind _outactors (Actor|GetAllActorsOfClass "/Game/ThirdPerson/Blueprints/BP_ThirdPersonCharacter.BP_ThirdPersonCharacter_C"))
  (Variables|Default|SetTimer%20Ref (Utilities|Array|Get(acopy) _outactors))
  (bind _outactors_2 (Actor|GetAllActorsOfClasswithTag "/Script/Engine.PostProcessVolume" "Glitch_Process"))
  (Variables|Default|SetGlitch_Post_Process_Volume (Utilities|Array|Get(acopy) _outactors_2)))

(fn ConstructionScript
  (|CallParentFunction))

(fn GetIsDetected
  (return (Variables|Default|GetIsDetected)))