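; Teleport station actor that lets either of the two player characters switch while standing inside its trigger box, showing a teleporter instruction widget.
; BeginPlay creates the hidden widget and caches the first instance of each character class.
; Box overlaps toggle the widget and set CanSwitch on the entering or leaving character, chosen by the Player1 tag.
; Tick also hides the widget whenever neither player can switch.
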(event OnComponentBeginOverlap(Box)
  (params (OverlappedComponent :type Primitive%20Component%20Object%20Reference) (OtherActor :type Actor%20Object%20Reference) (OtherComp :type Primitive%20Component%20Object%20Reference) (OtherBodyIndex :type Integer) (bFromSweep :type Boolean) (SweepResult :type Hit%20Result%20Structure%20%28by%20ref%29))
  (Widget|SetVisibility (Variables|Default|GetTele_widget) "Visible")
  (if (Actor|ActorHasTag OtherActor "Player1")
    (bind _asbp_third_person_character (Utilities|Casting|CastToBP_ThirdPersonCharacter OtherActor))
    (Variables|/Game/ThirdPerson/Blueprints/BP_ThirdPersonCharacter.BP_ThirdPersonCharacter_C|SetCan_Switch _asbp_third_person_character true)
    (else
      (bind _asbp_third_person_character_2 (Utilities|Casting|CastToBP_ThirdPersonCharacter2 OtherActor))
      (Variables|/Game/ThirdPerson/Blueprints/BP_ThirdPersonCharacter2.BP_ThirdPersonCharacter2_C|SetCan_Switch _asbp_third_person_character_2 true))))

(event OnComponentEndOverlap(Box)
  (params (OverlappedComponent :type Primitive%20Component%20Object%20Reference) (OtherActor :type Actor%20Object%20Reference) (OtherComp :type Primitive%20Component%20Object%20Reference) (OtherBodyIndex :type Integer))
  (Widget|SetVisibility (Variables|Default|GetTele_widget) "Hidden")
  (if (Actor|ActorHasTag OtherActor "Player1")
    (bind _asbp_third_person_character (Utilities|Casting|CastToBP_ThirdPersonCharacter OtherActor))
    (Variables|/Game/ThirdPerson/Blueprints/BP_ThirdPersonCharacter.BP_ThirdPersonCharacter_C|SetCan_Switch _asbp_third_person_character false)
    (else
      (bind _asbp_third_person_character_2 (Utilities|Casting|CastToBP_ThirdPersonCharacter2 OtherActor))
      (Variables|/Game/ThirdPerson/Blueprints/BP_ThirdPersonCharacter2.BP_ThirdPersonCharacter2_C|SetCan_Switch _asbp_third_person_character_2 false))))

(event EventBeginPlay
  (bind _returnvalue (UserInterface|CreateWidget "/Game/Blueprints/Alex_Assets/Blueprints/Teleporter_Inst.Teleporter_Inst_C"))
  (bind _output_get (Variables|Default|SetTele_widget _returnvalue))
  (UserInterface|Viewport|AddtoViewport _output_get 0)
  (Widget|SetVisibility (Variables|Default|GetTele_widget) "Hidden")
  (bind _outactors (Actor|GetAllActorsOfClass "/Game/ThirdPerson/Blueprints/BP_ThirdPersonCharacter.BP_ThirdPersonCharacter_C"))
  (Variables|Default|SetPlayer1 (Utilities|Array|Get(acopy) _outactors))
  (bind _outactors_2 (Actor|GetAllActorsOfClass "/Game/ThirdPerson/Blueprints/BP_ThirdPersonCharacter2.BP_ThirdPersonCharacter2_C"))
  (Variables|Default|SetPlayer2 (Utilities|Array|Get(acopy) _outactors_2)))

(event Collision|EventActorBeginOverlap
  (params (OtherActor :type Actor%20Object%20Reference)))

(event EventTick
  (params (DeltaSeconds :type Float%20%28single-precision%29))
  (if (and (== (Variables|/Game/ThirdPerson/Blueprints/BP_ThirdPersonCharacter2.BP_ThirdPersonCharacter2_C|GetCan_Switch (Variables|Default|GetPlayer2)) false) (== (Variables|/Game/ThirdPerson/Blueprints/BP_ThirdPersonCharacter.BP_ThirdPersonCharacter_C|GetCan_Switch (Variables|Default|GetPlayer1)) false))
    (CallFunction|HideInstructions)))

(fn ConstructionScript)

(fn HideInstructions
  (Widget|SetVisibility (Variables|Default|GetTele_widget) "Hidden"))