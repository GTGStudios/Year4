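; Level-end trigger actor that scores and ranks the player's run.
; On first overlap it stops the character's timer, disables input, shows the cursor and reveals the score widget.
; The score is the timer's value as a percentage of its BeginPlay value plus a diamond bonus, mapped to an S-to-F rank.
; AddDiamondScore raises that bonus and reveals up to three diamond images on the widget.
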(event OnComponentBeginOverlap(scoretrigger)
  (params (OverlappedComponent :type Primitive%20Component%20Object%20Reference) (OtherActor :type Actor%20Object%20Reference) (OtherComp :type Primitive%20Component%20Object%20Reference) (OtherBodyIndex :type Integer) (bFromSweep :type Boolean) (SweepResult :type Hit%20Result%20Structure%20%28by%20ref%29))
  (bind _returnvalue (Game|GetPlayerController 0))
  (Utilities|FlowControl|DoOnce false
    (:Completed
      (Variables|/Game/ThirdPerson/Blueprints/BP_ThirdPersonCharacter.BP_ThirdPersonCharacter_C|SetStartTime (Variables|Default|GetPlayer_time) false)
      (Input|DisableInput (Game|GetPlayerCharacter 0) _returnvalue)
      (Variables|/Script/Engine.PlayerController|SetbShowMouseCursor _returnvalue true)
      (Variables|Default|SetFinish%20Minutes (Variables|/Game/ThirdPerson/Blueprints/BP_ThirdPersonCharacter.BP_ThirdPersonCharacter_C|GetMinutes (Variables|Default|GetPlayer_time)))
      (Variables|Default|SetFinish%20Seconds (Variables|/Game/ThirdPerson/Blueprints/BP_ThirdPersonCharacter.BP_ThirdPersonCharacter_C|GetSeconds (Variables|Default|GetPlayer_time)))
      (Variables|Default|SetScore%20Calculation (+ (* (Variables|Default|GetFinish%20Minutes) 60) (Variables|Default|GetFinish%20Seconds)))
      (Variables|Default|SetFinal%20score (+ (* (/ (Variables|Default|GetScore%20Calculation) (Variables|Default|GetStarting%20time)) 1e+02) (Variables|Default|GetDiamonds%20score)))
      (if (>= (Variables|Default|GetFinal%20score) 90)
        (Variables|Default|SetRank "S")
        (Widget|SetVisibility (Variables|/Game/ThirdPerson/Blueprints/BP_ThirdPersonCharacter.BP_ThirdPersonCharacter_C|GetScore_Display (Variables|Default|GetPlayer_time)) "Visible" :!label _label)
        (elif (and (< (Variables|Default|GetFinal%20score) 90) (>= (Variables|Default|GetFinal%20score) 80))
          (Variables|Default|SetRank "A")
          (goto _label)
          (elif (and (< (Variables|Default|GetFinal%20score) 80) (>= (Variables|Default|GetFinal%20score) 70))
            (Variables|Default|SetRank "B")
            (goto _label)
            (elif (and (< (Variables|Default|GetFinal%20score) 70) (>= (Variables|Default|GetFinal%20score) 60))
              (Variables|Default|SetRank "C")
              (goto _label)
              (elif (and (< (Variables|Default|GetFinal%20score) 60) (>= (Variables|Default|GetFinal%20score) 50))
                (Variables|Default|SetRank "D")
                (goto _label)
                (elif (< (Variables|Default|GetFinal%20score) 50)
                  (Variables|Default|SetRank "F")
                  (goto _label))))))))))

(event EventBeginPlay
  (bind _outactors (Actor|GetAllActorsOfClass "/Game/ThirdPerson/Blueprints/BP_ThirdPersonCharacter.BP_ThirdPersonCharacter_C"))
  (Variables|Default|SetPlayer_time (Utilities|Array|Get(acopy) _outactors))
  (Variables|Default|SetStarting%20time (Math|Conversions|ToFloat(Integer) (+ (Variables|/Game/ThirdPerson/Blueprints/BP_ThirdPersonCharacter.BP_ThirdPersonCharacter_C|GetSeconds (Variables|Default|GetPlayer_time)) (* (Variables|/Game/ThirdPerson/Blueprints/BP_ThirdPersonCharacter.BP_ThirdPersonCharacter_C|GetMinutes (Variables|Default|GetPlayer_time)) 60))))
  (bind _foundwidgets (Widget|GetAllWidgetsOfClass "/Game/Blueprints/Alex_Assets/Blueprints/Score_displpay.Score_displpay_C" true))
  (Variables|Default|SetScore_Display (Utilities|Array|Get(acopy) _foundwidgets)))

(event Collision|EventActorBeginOverlap
  (params (OtherActor :type Actor%20Object%20Reference)))

(event EventTick
  (params (DeltaSeconds :type Float%20%28single-precision%29)))

(fn ConstructionScript)

(fn AddDiamondScore
  (bind _player_time (Variables|Default|GetPlayer_time))
  (bind _score_display (Variables|/Game/ThirdPerson/Blueprints/BP_ThirdPersonCharacter.BP_ThirdPersonCharacter_C|GetScore_Display _player_time))
  (Variables|Default|SetDiamonds%20score (+ (Variables|Default|GetDiamonds%20score) 10))
  (if (== (Variables|Default|GetDiamonds%20score) 10)
    (Widget|SetVisibility (Variables|/Game/Blueprints/Alex_Assets/Blueprints/Score_displpay.Score_displpay_C|GetDiamonsImage1 _score_display) "Visible")
    (elif (== (Variables|Default|GetDiamonds%20score) 20)
      (Widget|SetVisibility (Variables|/Game/Blueprints/Alex_Assets/Blueprints/Score_displpay.Score_displpay_C|GetDiamonsImage2 _score_display) "Visible")
      (elif (== (Variables|Default|GetDiamonds%20score) 30)
        (Widget|SetVisibility (Variables|/Game/Blueprints/Alex_Assets/Blueprints/Score_displpay.Score_displpay_C|GetDiamonsImage3 _score_display) "Visible")))))