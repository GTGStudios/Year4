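; Interactable server rack that starts time for the player, judging by its name and the StartTime flag it sets.
; BeginPlay caches the first third-person character and the first Hack_Station_Observer found in the level.
; StartInteract runs once, setting StartTime on the character, firing the observer's HackPickupEvent and switching the rack's second material slot to Neon.
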(event EventBeginPlay
  (bind _outactors (Actor|GetAllActorsOfClass "/Game/ThirdPerson/Blueprints/BP_ThirdPersonCharacter.BP_ThirdPersonCharacter_C"))
  (Variables|Default|SetCharRef (Utilities|Array|Get(acopy) _outactors))
  (bind _outactors_2 (Actor|GetAllActorsOfClass "/Game/Blueprints/Alex_Assets/Blueprints/Hack_Station_Observer.Hack_Station_Observer_C"))
  (Variables|Default|SetObs_ref (Utilities|Array|Get(acopy) _outactors_2)))

(event Collision|EventActorBeginOverlap
  (params (OtherActor :type Actor%20Object%20Reference)))

(event EventTick
  (params (DeltaSeconds :type Float%20%28single-precision%29)))

(event EventStartInteract
  (params (Player :type Character%20Object%20Reference))
  (Utilities|FlowControl|DoOnce false
    (:Completed
      (Variables|/Game/ThirdPerson/Blueprints/BP_ThirdPersonCharacter.BP_ThirdPersonCharacter_C|SetStartTime (Variables|Default|GetCharRef) true)
      (Default|HackPickupEvent (Variables|Default|GetObs_ref))
      (Rendering|Material|SetMaterial (Variables|Default|GetServerRack) 1 "/Game/3D_Assets/LabAssets/SlidingDoors/Mats/Neon.Neon"))))

(fn ConstructionScript)