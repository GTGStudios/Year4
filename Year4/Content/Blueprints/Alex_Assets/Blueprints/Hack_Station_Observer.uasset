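; Hack station observer that counts hack pickups and relays the running total to doors and the level's elevator.
; On BeginPlay it caches the first BP_Elevator found in the world.
; Hack_Pickup_Event increments PickupNum, then loops over DoorArray, asking each door to check whether it should open and updating the elevator light on every iteration.
; A BP_ElevatorDoors lookup is left unconnected and never runs.
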(event Custom|Hack_Pickup_Event
  (Variables|Default|SetPickup_num (+ (Variables|Default|GetPickup_num) 1))
  (for _array_element (Variables|Default|GetDoor_Array)
    (Default|CheckIfshouldOpen _array_element (Variables|Default|GetPickup_num))
    (Default|AlertElevatorLight (Variables|Default|GetElevator) (Variables|Default|GetPickup_num))))

(event EventBeginPlay
  (bind _outactors (Actor|GetAllActorsOfClass "/Game/BP_Elevator.BP_Elevator_C"))
  (Variables|Default|SetElevator (Utilities|Array|Get(acopy) _outactors)))

(event Collision|EventActorBeginOverlap
  (params (OtherActor :type Actor%20Object%20Reference)))

(event EventTick
  (params (DeltaSeconds :type Float%20%28single-precision%29)))

(fn ConstructionScript)