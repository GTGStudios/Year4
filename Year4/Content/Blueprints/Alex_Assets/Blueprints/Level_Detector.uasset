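; Level detector Blueprint that records which level is currently loaded in the Level_manager game instance.
; On BeginPlay it compares the current level name against a hardcoded chain of five known map names.
; A match sets LevelIndicator to that level's label, usually a shortened name, and prints it to screen.
; Unrecognised levels leave the indicator unchanged.
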(event EventBeginPlay
  (bind _returnvalue (Game|GetCurrentLevelName true))
  (if (Utilities|Enum|Equal(Enum) _returnvalue "Reid")
    (bind _aslevel_manager (Utilities|Casting|CastToLevel_manager (Game|GetGameInstance)))
    (bind _output_get (Variables|/Game/Blueprints/Level_manager.Level_manager_C|SetLevel_Indicator _aslevel_manager _returnvalue))
    (Development|PrintString _output_get)
    (elif (Utilities|Enum|Equal(Enum) _returnvalue "Scientist_Grey_Box_lvl1")
      (bind _aslevel_manager_2 (Utilities|Casting|CastToLevel_manager (Game|GetGameInstance)))
      (bind _output_get_2 (Variables|/Game/Blueprints/Level_manager.Level_manager_C|SetLevel_Indicator _aslevel_manager_2 "Sci Lvl1"))
      (Development|PrintString _output_get_2)
      (elif (Utilities|Enum|Equal(Enum) _returnvalue "Scavanger_Hunt_Grey_Box")
        (bind _aslevel_manager_3 (Utilities|Casting|CastToLevel_manager (Game|GetGameInstance)))
        (bind _output_get_3 (Variables|/Game/Blueprints/Level_manager.Level_manager_C|SetLevel_Indicator _aslevel_manager_3 "Hunt"))
        (Development|PrintString _output_get_3)
        (elif (Utilities|Enum|Equal(Enum) _returnvalue "TeleporterLab")
          (bind _aslevel_manager_4 (Utilities|Casting|CastToLevel_manager (Game|GetGameInstance)))
          (bind _output_get_4 (Variables|/Game/Blueprints/Level_manager.Level_manager_C|SetLevel_Indicator _aslevel_manager_4 "Teleporter"))
          (Development|PrintString _output_get_4)
          (elif (Utilities|Enum|Equal(Enum) _returnvalue "ConstructionRoom")
            (bind _aslevel_manager_5 (Utilities|Casting|CastToLevel_manager (Game|GetGameInstance)))
            (bind _output_get_5 (Variables|/Game/Blueprints/Level_manager.Level_manager_C|SetLevel_Indicator _aslevel_manager_5 "Construction"))
            (Development|PrintString _output_get_5)))))))

(fn ConstructionScript)