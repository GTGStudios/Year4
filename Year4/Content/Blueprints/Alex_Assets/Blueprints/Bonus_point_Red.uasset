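; Red bonus point pickup that adds to the diamond score when interacted with.
; On BeginPlay it caches the first third-person character and the first Final_score actor found in the level.
; StartInteract calls AddDiamondScore on that score actor, then destroys the pickup.
; The cached character is used only by a disconnected node that would set StartTime, so that logic never runs.
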(event EventBeginPlay
  (bind _outactors (Actor|GetAllActorsOfClass "/Game/ThirdPerson/Blueprints/BP_ThirdPersonCharacter.BP_ThirdPersonCharacter_C"))
  (Variables|Default|SetCharRef (Utilities|Array|Get(acopy) _outactors))
  (bind _outactors_2 (Actor|GetAllActorsOfClass "/Game/Blueprints/Alex_Assets/Blueprints/Final_score.Final_score_C"))
  (Variables|Default|SetScore (Utilities|Array|Get(acopy) _outactors_2)))

(event Collision|EventActorBeginOverlap
  (params (OtherActor :type Actor%20Object%20Reference)))

(event EventTick
  (params (DeltaSeconds :type Float%20%28single-precision%29)))

(event EventStartInteract
  (params (Player :type Character%20Object%20Reference))
  (Default|AddDiamondScore (Variables|Default|GetScore))
  (Actor|DestroyActor))

(fn ConstructionScript)