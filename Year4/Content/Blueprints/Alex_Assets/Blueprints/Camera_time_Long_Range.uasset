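; Rotating security camera that costs the player time when its PawnSensing spots a pawn.
; A sighting sets StartTime on the first BP_ThirdPersonCharacter found at BeginPlay.
; If Activated, it also deducts Seconds from that character and plays an alert, then clears StartTime after a short delay.
; An Ice_Block overlapping the Box pauses the RotatingMovement until it leaves, while sensing stays live.
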(event OnSeePawn(PawnSensing)
  (params (Pawn :type Pawn%20Object%20Reference))
  (Variables|/Game/ThirdPerson/Blueprints/BP_ThirdPersonCharacter.BP_ThirdPersonCharacter_C|SetStartTime (Variables|Default|GetTimeRef) true)
  (if (Variables|Default|GetActivated)
    (Utilities|FlowControl|Sequence
      (:then_0
        (Variables|/Game/ThirdPerson/Blueprints/BP_ThirdPersonCharacter.BP_ThirdPersonCharacter_C|SetSeconds (Variables|Default|GetTimeRef) (- (Variables|/Game/ThirdPerson/Blueprints/BP_ThirdPersonCharacter.BP_ThirdPersonCharacter_C|GetSeconds (Variables|Default|GetTimeRef)) 5))
        (Audio|PlaySound2D "/Game/Blueprints/Alex_Assets/Sounds/alert_mk1.alert_mk1" 1.0 1.0 0.0 0 0)
        (Utilities|FlowControl|Delay 1.0)
        (Variables|/Game/ThirdPerson/Blueprints/BP_ThirdPersonCharacter.BP_ThirdPersonCharacter_C|SetStartTime (Variables|Default|GetTimeRef) false)))))

(event OnComponentBeginOverlap(Box)
  (params (OverlappedComponent :type Primitive%20Component%20Object%20Reference) (OtherActor :type Actor%20Object%20Reference) (OtherComp :type Primitive%20Component%20Object%20Reference) (OtherBodyIndex :type Integer) (bFromSweep :type Boolean) (SweepResult :type Hit%20Result%20Structure%20%28by%20ref%29))
  (Utilities|Casting|CastToIce_Block OtherActor)
  (Components|Activation|Deactivate (Variables|Default|GetRotatingMovement)))

(event OnComponentEndOverlap(Box)
  (params (OverlappedComponent :type Primitive%20Component%20Object%20Reference) (OtherActor :type Actor%20Object%20Reference) (OtherComp :type Primitive%20Component%20Object%20Reference) (OtherBodyIndex :type Integer))
  (Utilities|Casting|CastToIce_Block OtherActor)
  (Components|Activation|Activate (Variables|Default|GetRotatingMovement) false))

(event EventBeginPlay
  (bind _outactors (Actor|GetAllActorsOfClass "/Game/ThirdPerson/Blueprints/BP_ThirdPersonCharacter.BP_ThirdPersonCharacter_C"))
  (Variables|Default|SetTimeRef (Utilities|Array|Get(acopy) _outactors)))

(event Collision|EventActorBeginOverlap
  (params (OtherActor :type Actor%20Object%20Reference)))

(fn ConstructionScript)