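; Camera actor that penalizes the player's time when its PawnSensing component sees a pawn.
; BeginPlay caches the first BP_ThirdPersonCharacter found, and each OnSeePawn event subtracts five from that character's Seconds.
; The one-second retriggerable delay sits on a separate sequence branch with nothing after it, so it does not throttle the penalty.
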(event OnSeePawn(PawnSensing)
  (params (Pawn :type Pawn%20Object%20Reference))
  (Utilities|FlowControl|Sequence
    (:then_0
      (Variables|/Game/ThirdPerson/Blueprints/BP_ThirdPersonCharacter.BP_ThirdPersonCharacter_C|SetSeconds (Variables|Default|GetTimeRef) (- (Variables|/Game/ThirdPerson/Blueprints/BP_ThirdPersonCharacter.BP_ThirdPersonCharacter_C|GetSeconds (Variables|Default|GetTimeRef)) 5)))
    (:then_1
      (Utilities|FlowControl|RetriggerableDelay 1.0))))

(event EventBeginPlay
  (bind _outactors (Actor|GetAllActorsOfClass "/Game/ThirdPerson/Blueprints/BP_ThirdPersonCharacter.BP_ThirdPersonCharacter_C"))
  (Variables|Default|SetTimeRef (Utilities|Array|Get(acopy) _outactors)))

(event Collision|EventActorBeginOverlap
  (params (OtherActor :type Actor%20Object%20Reference)))

(event EventTick
  (params (DeltaSeconds :type Float%20%28single-precision%29)))

(fn ConstructionScript)