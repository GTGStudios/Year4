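; Laser wall actor that can blink on and off as a timed obstacle, with a looping toggle enabled by the Disapear flag.
; Tick feeds a three-second Delay into a FlipFlop, which alternately hides and shows the laser cylinder, switches its and the box's collision, and pauses or resumes the wall sound.
; The sound stops at BeginPlay when PlaySound is false, and a StopSound function also stops it.
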(event EventBeginPlay
  (if (not (Variables|Default|GetPlay%20sound))
    (Audio|Components|Audio|Stop (Variables|Default|GetLaser_wall_sound))))

(event Collision|EventActorBeginOverlap
  (params (OtherActor :type Actor%20Object%20Reference)))

(event EventTick
  (params (DeltaSeconds :type Float%20%28single-precision%29))
  (bind _lasercylinder3 (Variables|Default|GetLaserCylinder3))
  (bind _laser_wall_sound (Variables|Default|GetLaser_wall_sound))
  (if (Variables|Default|GetDisapear)
    (Utilities|FlowControl|Delay 3.0)
    (Utilities|FlowControl|FlipFlop
      (:A
        (Development|SetHiddeninGame _lasercylinder3 true false)
        (Collision|SetCollisionEnabled _lasercylinder3 "NoCollision")
        (Class|AudioComponent|SetPaused _laser_wall_sound true))
      (:B
        (Development|SetHiddeninGame _lasercylinder3 false false)
        (Collision|SetCollisionEnabled _lasercylinder3 "QueryAndPhysics")
        (Class|AudioComponent|SetPaused _laser_wall_sound false)))))

(fn ConstructionScript)

(fn StopSound
  (Audio|Components|Audio|Stop (Variables|Default|GetLaser_wall_sound)))