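; Tutorial trigger box that pauses play to show an instruction the first time it is overlapped.
; On overlap it clears the Tutorial_Manager text, shows the character's tutorial overlay, freezes both characters with zero time dilation and clears StartTime.
; A looping timer types the instruction into the manager one letter at a time.
; End overlap clears ShowText so the box does not show again; resuming play is handled outside this Blueprint.
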(event OnComponentBeginOverlap(Box)
  (params (OverlappedComponent :type Primitive%20Component%20Object%20Reference) (OtherActor :type Actor%20Object%20Reference) (OtherComp :type Primitive%20Component%20Object%20Reference) (OtherBodyIndex :type Integer) (bFromSweep :type Boolean) (SweepResult :type Hit%20Result%20Structure%20%28by%20ref%29))
  (CallFunction|DisableWidget)
  (if (Variables|Default|GetShowText)
    (Default|ShowOverlay (Variables|/Game/ThirdPerson/Blueprints/BP_ThirdPersonCharacter.BP_ThirdPersonCharacter_C|GetTutorial_box (Variables|Default|GetCharRef)))
    (Variables|/Game/Blueprints/Alex_Assets/Blueprints/Tutorial_Manager.Tutorial_Manager_C|SetUnpauseInst (Variables|Default|GetManager) (Variables|Default|GetPause))
    (bind _returnvalue (Utilities|Time|SetTimerbyEvent (delegate Custom|Type_Text) 0.1 true))
    (Variables|/Script/Engine.Actor|SetCustomTimeDilation (Variables|Default|GetCharRef) 0.0)
    (Variables|/Script/Engine.Actor|SetCustomTimeDilation (Variables|Default|GetChar2_Ref) 0.0)
    (Variables|/Game/ThirdPerson/Blueprints/BP_ThirdPersonCharacter.BP_ThirdPersonCharacter_C|SetStartTime (Variables|Default|GetCharRef) false)))

(event OnComponentEndOverlap(Box)
  (params (OverlappedComponent :type Primitive%20Component%20Object%20Reference) (OtherActor :type Actor%20Object%20Reference) (OtherComp :type Primitive%20Component%20Object%20Reference) (OtherBodyIndex :type Integer))
  (if (Variables|Default|GetShowText)
    (Variables|Default|SetShowText false)))

(event Custom|Type_Text
  (Variables|/Game/Blueprints/Alex_Assets/Blueprints/Tutorial_Manager.Tutorial_Manager_C|SetTut_Text (Variables|Default|GetManager) (Utilities|String|Append (Variables|/Game/Blueprints/Alex_Assets/Blueprints/Tutorial_Manager.Tutorial_Manager_C|GetTut_Text (Variables|Default|GetManager)) (Utilities|Array|Get(acopy) (Utilities|String|GetCharacterArrayfromString (Variables|Default|GetNew_instructions)) (Variables|Default|GetIndex))))
  (bind _result (Math|Integer|IncrementInt (Variables|Default|GetIndex))
    (:%20%20
      (if (== _result (Utilities|Array|Length (Utilities|String|GetCharacterArrayfromString (Variables|Default|GetNew_instructions))))
        (Utilities|Time|ClearandInvalidateTimerbyHandle (stale OnComponentBeginOverlap(Box) _returnvalue))))))

(event EventBeginPlay
  (bind _outactors (Actor|GetAllActorsOfClass "/Game/Blueprints/Alex_Assets/Blueprints/Tutorial_Manager.Tutorial_Manager_C"))
  (Variables|Default|SetManager (Utilities|Array|Get(acopy) _outactors))
  (bind _outactors_2 (Actor|GetAllActorsOfClass "/Game/ThirdPerson/Blueprints/BP_ThirdPersonCharacter.BP_ThirdPersonCharacter_C"))
  (Variables|Default|SetCharRef (Utilities|Array|Get(acopy) _outactors_2))
  (bind _outactors_3 (Actor|GetAllActorsOfClass "/Game/ThirdPerson/Blueprints/BP_ThirdPersonCharacter2.BP_ThirdPersonCharacter2_C"))
  (Variables|Default|SetChar2_Ref (Utilities|Array|Get(acopy) _outactors_3))
  (bind _foundwidgets (Widget|GetAllWidgetsOfClass "/Game/Blueprints/Alex_Assets/Blueprints/Tutorial_inst.Tutorial_inst_C" true))
  (Variables|Default|Settutorial%20widge (Utilities|Array|Get(acopy) _foundwidgets)))

(event Collision|EventActorBeginOverlap
  (params (OtherActor :type Actor%20Object%20Reference)))

(event EventTick
  (params (DeltaSeconds :type Float%20%28single-precision%29)))

(fn ConstructionScript)

(fn DisableWidget
  (Variables|/Game/Blueprints/Alex_Assets/Blueprints/Tutorial_Manager.Tutorial_Manager_C|SetTut_Text (Variables|Default|GetManager) (Variables|Default|GetInst_clear))
  (Variables|/Game/Blueprints/Alex_Assets/Blueprints/Tutorial_Manager.Tutorial_Manager_C|SetUnpauseInst (Variables|Default|GetManager) (Variables|Default|GetInst_clear)))