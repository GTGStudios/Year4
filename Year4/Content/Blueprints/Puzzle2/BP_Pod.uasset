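; Lights Out-style puzzle pod for Puzzle2 that toggles itself and its neighbors when a player character steps into its box trigger.
; An overlap by either of the two third-person character classes flips the On state of the pod and every pod in its Adjacentpod array, without cascading further.
; The cube swaps between on and off materials on each toggle, at BeginPlay and redundantly every Tick.
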(event OnComponentBeginOverlap(Box)
  (params (OverlappedComponent :type Primitive%20Component%20Object%20Reference) (OtherActor :type Actor%20Object%20Reference) (OtherComp :type Primitive%20Component%20Object%20Reference) (OtherBodyIndex :type Integer) (bFromSweep :type Boolean) (SweepResult :type Hit%20Result%20Structure%20%28by%20ref%29))
  (bind _returnvalue (Utilities|GetClass OtherActor))
  (Development|PrintString "Hello")
  (if (== _returnvalue "/Game/ThirdPerson/Blueprints/BP_ThirdPersonCharacter.BP_ThirdPersonCharacter_C")
    (if (Variables|Default|GetOn) :!label _label
      (Variables|Default|SetOn false)
      (CallFunction|TurnOff)
      (else
        (Variables|Default|SetOn true)
        (CallFunction|TurnON)))
    (for _array_element (Variables|Default|Getadjacentpod)
      (if (Variables|BP_Pod_C|GetOn _array_element)
        (Variables|BP_Pod_C|SetOn _array_element false)
        (CallFunction|TurnOff _array_element)
        (else
          (Variables|BP_Pod_C|SetOn _array_element true)
          (CallFunction|TurnON _array_element))))
    (elif (== _returnvalue "/Game/ThirdPerson/Blueprints/BP_ThirdPersonCharacter2.BP_ThirdPersonCharacter2_C")
      (goto _label))))

(event Custom|TurnOff
  (Rendering|Material|SetMaterial (Variables|Default|GetCube) 0 "/Game/Blueprints/Puzzle2/M_ISOFF.M_ISOFF"))

(event Custom|TurnON
  (Rendering|Material|SetMaterial (Variables|Default|GetCube) 0 "/Game/Blueprints/Puzzle2/M_ISON.M_ISON"))

(event EventBeginPlay
  (bind _cube (Variables|Default|GetCube))
  (if (Variables|Default|GetOn)
    (Rendering|Material|SetMaterial _cube 0 "/Game/Blueprints/Puzzle2/M_ISON.M_ISON")
    (else
      (Rendering|Material|SetMaterial _cube 0 "/Game/Blueprints/Puzzle2/M_ISOFF.M_ISOFF"))))

(event Collision|EventActorBeginOverlap
  (params (OtherActor :type Actor%20Object%20Reference)))

(event EventTick
  (params (DeltaSeconds :type Float%20%28single-precision%29))
  (bind _cube (Variables|Default|GetCube))
  (if (Variables|Default|GetOn)
    (Rendering|Material|SetMaterial _cube 0 "/Game/Blueprints/Puzzle2/M_ISON.M_ISON")
    (else
      (Rendering|Material|SetMaterial _cube 0 "/Game/Blueprints/Puzzle2/M_ISOFF.M_ISOFF"))))

(fn ConstructionScript)