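; BP_PPodManager is a puzzle manager that tracks a set of pods and removes designated objects once all of them are on.
; Pods are added to PodList through AddPod.
; CheckIfOn counts the pods whose On flag is set; when the count reaches the list length, it prints "Solved" and destroys every actor in DisbaleObj, otherwise it resets the count.
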(event Custom|CheckIfOn
  (for _array_element (Variables|Default|GetPodList)
    (if (Variables|/Game/Blueprints/Puzzle2/BP_PPod.BP_PPod_C|GetOn _array_element)
      (Variables|Default|SetCount (+ (Variables|Default|GetCount) 1))))
  (if (>= (Variables|Default|GetCount) (Utilities|Array|Length (Variables|Default|GetPodList)))
    (Development|PrintString "Solved")
    (for _array_element_2 (Variables|Default|GetDisbale%20Obj)
      (Actor|DestroyActor _array_element_2))
    (else
      (Variables|Default|SetCount 0))))

(event Custom|AddPod
  (params (Pod1 :type BP%20P%20Pod%20Object%20Reference))
  (Utilities|Array|Add (Variables|Default|GetPodList) Pod1))

(fn ConstructionScript)