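; BP_PodManager is a puzzle manager that checks whether every pod in PodList is switched on.
; Its CheckIfOn event, with no caller in this graph, counts the pods whose On flag is true.
; When the count reaches the list length, it prints a solved message and destroys every actor in DisbaleObj.
; Otherwise it resets the count to zero for the next check.
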(event Custom|CheckIfOn
  (for _array_element (Variables|Default|GetPodList)
    (if (Variables|/Game/Blueprints/Puzzle2/BP_Pod.BP_Pod_C|GetOn _array_element)
      (Variables|Default|SetCount (+ (Variables|Default|GetCount) 1))))
  (if (>= (Variables|Default|GetCount) (Utilities|Array|Length (Variables|Default|GetPodList)))
    (Development|PrintString "Solved")
    (for _array_element_2 (Variables|Default|GetDisbale%20Obj)
      (Actor|DestroyActor _array_element_2))
    (else
      (Variables|Default|SetCount 0))))

(event EventBeginPlay)

(event Collision|EventActorBeginOverlap
  (params (OtherActor :type Actor%20Object%20Reference)))

(event EventTick
  (params (DeltaSeconds :type Float%20%28single-precision%29)))

(fn ConstructionScript)