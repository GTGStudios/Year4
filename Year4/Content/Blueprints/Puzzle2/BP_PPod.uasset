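; BP_PPod is a puzzle pressure pad that switches on while either of two third-person characters or a box rests on it.
; Begin play and every Box overlap begin or end rescan the overlapping actors, using IsOn as a temporary found flag.
; TurnON and TurnOff swap the Cube's material, set On, and ask PodManager, where the pad registers at begin play, to re-check.
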(event OnComponentBeginOverlap(Box)
  (params (OverlappedComponent :type Primitive%20Component%20Object%20Reference) (OtherActor :type Actor%20Object%20Reference) (OtherComp :type Primitive%20Component%20Object%20Reference) (OtherBodyIndex :type Integer) (bFromSweep :type Boolean) (SweepResult :type Hit%20Result%20Structure%20%28by%20ref%29))
  (CallFunction|Checkifon))

(event OnComponentEndOverlap(Box)
  (params (OverlappedComponent :type Primitive%20Component%20Object%20Reference) (OtherActor :type Actor%20Object%20Reference) (OtherComp :type Primitive%20Component%20Object%20Reference) (OtherBodyIndex :type Integer))
  (CallFunction|Checkifon))

(event Custom|CheckifOn
  (for _array_element (Collision|GetOverlappingActors (Variables|Default|GetBox) 0 :!class /Script/Engine.PrimitiveComponent)
    (if (not (Variables|Default|GetIsOn))
      (if (Math|Boolean|ORBoolean (== _array_element "/Game/ThirdPerson/Blueprints/BP_ThirdPersonCharacter.BP_ThirdPersonCharacter_C") (== _array_element "/Game/ThirdPerson/Blueprints/BP_ThirdPersonCharacter2.BP_ThirdPersonCharacter2_C") (== _array_element "/Game/Blueprints/BP_box.BP_box_C"))
        (CallFunction|TurnON)
        (Variables|Default|SetIsOn true))))
  (if (Variables|Default|GetIsOn)
    (Variables|Default|SetIsOn false)
    (else
      (CallFunction|TurnOff))))

(event Custom|TurnOff
  (Rendering|Material|SetMaterial (Variables|Default|GetCube) 0 "/Game/Blueprints/CircuitPuzzle/gram7.gram7")
  (Variables|Default|SetOn false)
  (Default|Checkifon (Variables|Default|GetPodManager)))

(event Custom|TurnON
  (Rendering|Material|SetMaterial (Variables|Default|GetCube) 0 "/Game/Blueprints/CircuitPuzzle/gram0.gram0")
  (Variables|Default|SetOn true)
  (Default|Checkifon (Variables|Default|GetPodManager)))

(event EventBeginPlay
  (bind _podmanager (Variables|Default|GetPodManager))
  (CallFunction|Checkifon)
  (Default|AddPod _podmanager self)
  (Default|Checkifon _podmanager))

(event Collision|EventActorBeginOverlap
  (params (OtherActor :type Actor%20Object%20Reference)))

(fn ConstructionScript)