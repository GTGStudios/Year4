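; Trigger actor that advances the player's mission the first time anything overlaps its Trigger component.
; At BeginPlay it caches the first BP_ThirdPersonCharacter in the level as Player1.
; A DoOnce-gated overlap passes NewMissionToSet to that character's UpdateMission, without checking which actor overlapped.
; It then casts Target's ObjectRef to WP_Mission and calls UpdateMissionWB to refresh it.
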(event OnComponentBeginOverlap(Trigger)
  (params (OverlappedComponent :type Primitive%20Component%20Object%20Reference) (OtherActor :type Actor%20Object%20Reference) (OtherComp :type Primitive%20Component%20Object%20Reference) (OtherBodyIndex :type Integer) (bFromSweep :type Boolean) (SweepResult :type Hit%20Result%20Structure%20%28by%20ref%29))
  (bind _target (Variables|Default|GetTarget))
  (bind _objectref (Variables|/Game/Blueprints/Checklist/WP_Mission.WP_Mission_C|GetObjectRef _target))
  (Utilities|FlowControl|DoOnce false
    (:Completed
      (Default|UpdateMission (Variables|Default|GetPlayer1) (Variables|Default|GetNewMissionToSet))
      (Utilities|Casting|CastToWP_Mission _objectref)
      (Default|UpdateMissionWB _objectref))))

(event EventBeginPlay
  (bind _outactors (Actor|GetAllActorsOfClass "/Game/ThirdPerson/Blueprints/BP_ThirdPersonCharacter.BP_ThirdPersonCharacter_C"))
  (Variables|Default|SetPlayer1 (Utilities|Array|Get(acopy) _outactors)))

(event Collision|EventActorBeginOverlap
  (params (OtherActor :type Actor%20Object%20Reference)))

(event EventTick
  (params (DeltaSeconds :type Float%20%28single-precision%29)))

(fn ConstructionScript)