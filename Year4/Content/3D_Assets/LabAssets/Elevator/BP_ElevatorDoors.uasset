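; BP_ElevatorDoors is an elevator door actor whose two doors slide open on overlap once it is unlocked.
; CheckIfshouldOpen sets the Shouldopen flag when the number passed in reaches OpenNum.
; With the flag set, Box overlaps drive the right door and Box1 overlaps the left, each through its own timeline with swept relative moves.
; The graph contains no closing or flag-reset logic.
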(event OnComponentBeginOverlap(Box)
  (params (OverlappedComponent :type Primitive%20Component%20Object%20Reference) (OtherActor :type Actor%20Object%20Reference) (OtherComp :type Primitive%20Component%20Object%20Reference) (OtherBodyIndex :type Integer) (bFromSweep :type Boolean) (SweepResult :type Hit%20Result%20Structure%20%28by%20ref%29))
  (if (Variables|Default|GetShouldopen)
    (bind _rightdooropen (Timeline|RightDoor Play)
      (:Update
        (Transformation|SetRelativeLocation (Variables|Default|GetElevatorDoors_RightDoor) _rightdooropen true false)))))

(event OnComponentBeginOverlap(Box1)
  (params (OverlappedComponent :type Primitive%20Component%20Object%20Reference) (OtherActor :type Actor%20Object%20Reference) (OtherComp :type Primitive%20Component%20Object%20Reference) (OtherBodyIndex :type Integer) (bFromSweep :type Boolean) (SweepResult :type Hit%20Result%20Structure%20%28by%20ref%29))
  (if (Variables|Default|GetShouldopen)
    (bind _leftdooropen (Timeline|LeftDoor Play)
      (:Update
        (Transformation|SetRelativeLocation (Variables|Default|GetElevatorDoors_LeftDoor) _leftdooropen true false)))))

(fn ConstructionScript)

(fn CheckIfshouldOpen
  (params (Number :type Integer))
  (if (>= Number (Variables|Default|GetOpenNum))
    (Variables|Default|SetShouldopen true)))