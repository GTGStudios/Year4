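; BP_FloatingStool is a lab prop actor that makes a stool float up and down in place.
; Each Tick sets the FloaterStool component's relative location from the Stool vector, adding a sine-wave offset on Z.
; The wave uses degree-based sine of the actor's time since creation, with BobbingSpeed and BobbingDistance controlling rate and amplitude.
; BeginPlay only re-applies the component's current relative location.
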(event EventBeginPlay
  (bind _floater_stool (Variables|Default|Getfloater_Stool))
  (Transformation|SetRelativeLocation _floater_stool (Variables|/Script/Engine.SceneComponent|GetRelativeLocation _floater_stool) false false))

(event Collision|EventActorBeginOverlap
  (params (OtherActor :type Actor%20Object%20Reference)))

(event EventTick
  (params (DeltaSeconds :type Float%20%28single-precision%29))
  (bind _stool (Variables|Default|GetStool))
  (bind (_x _y _z) (Math|Vector|BreakVector _stool))
  (Transformation|SetRelativeLocation (Variables|Default|Getfloater_Stool) (Math|Vector|MakeVector _x _y (+ _z (* (Math|Trig|Sin(Degrees) (* (Actor|GetGameTimeSinceCreation) (Variables|Default|GetBobbingSpeed))) (Variables|Default|GetBobbingDistance)))) false false))

(fn ConstructionScript)