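; Elevator that moves after an overlap with its trigger box and a short delay, alternating direction on each ride.
; The Up flag selects one of two timelines driving the Elevator1 mesh location, with a FlipFlop switching between play and reverse.
; An invisible Cube has collision only during rides, and Move and RidesDone gate re-triggering until the box is exited.
; AlertElevatorLight turns one of three material slots green by pickup number.
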(event OnComponentBeginOverlap(Box)
  (params (OverlappedComponent :type Primitive%20Component%20Object%20Reference) (OtherActor :type Actor%20Object%20Reference) (OtherComp :type Primitive%20Component%20Object%20Reference) (OtherBodyIndex :type Integer) (bFromSweep :type Boolean) (SweepResult :type Hit%20Result%20Structure%20%28by%20ref%29))
  (Utilities|FlowControl|Delay 0.5)
  (if (Variables|Default|Getmove)
    (Variables|Default|Setmove false)
    (Variables|Default|SetRides%20Done false)
    (Collision|SetCollisionEnabled (Variables|Default|GetCube) "QueryAndPhysics")
    (if (Variables|Default|GetUp?)
      (Utilities|FlowControl|FlipFlop
        (:A
          (bind _newtrack_0 (Timeline|Timeline Play)
            (:Update
              (Transformation|SetRelativeLocation (Variables|Default|GetElevator1) _newtrack_0 false false))
            (:Finished
              (Variables|Default|SetRides%20Done true)
              (Collision|SetCollisionEnabled (Variables|Default|GetCube) "NoCollision"))))
        (:B
          (Timeline|Timeline Reverse)))
      (else
        (Utilities|FlowControl|FlipFlop
          (:A
            (bind _newtrack_0_2 (Timeline|Timeline_0 Play)
              (:Update
                (Transformation|SetRelativeLocation (Variables|Default|GetElevator1) _newtrack_0_2 false false))
              (:Finished
                (Variables|Default|SetRides%20Done true)
                (Collision|SetCollisionEnabled (Variables|Default|GetCube) "NoCollision"))))
          (:B
            (Timeline|Timeline_0 Reverse)))))))

(event OnComponentEndOverlap(Box)
  (params (OverlappedComponent :type Primitive%20Component%20Object%20Reference) (OtherActor :type Actor%20Object%20Reference) (OtherComp :type Primitive%20Component%20Object%20Reference) (OtherBodyIndex :type Integer))
  (if (Variables|Default|GetRides%20Done)
    (Utilities|FlowControl|Delay 1.0)
    (Variables|Default|Setmove true)))

(event EventBeginPlay
  (bind _cube (Variables|Default|GetCube))
  (Rendering|SetVisibility _cube false false)
  (Collision|SetCollisionEnabled _cube "NoCollision"))

(fn ConstructionScript)

(fn AlertElevatorLight
  (params (Pickup :type Integer))
  (if (== Pickup 1)
    (Rendering|Material|SetMaterial (Variables|Default|GetElevator1) 10 "/Game/Materials/Emission/greenEmission.greenEmission")
    (elif (== Pickup 2)
      (Rendering|Material|SetMaterial (Variables|Default|GetElevator1) 9 "/Game/Materials/Emission/greenEmission.greenEmission")
      (elif (== Pickup 3)
        (Rendering|Material|SetMaterial (Variables|Default|GetElevator1) 0 "/Game/Materials/Emission/greenEmission.greenEmission")))))